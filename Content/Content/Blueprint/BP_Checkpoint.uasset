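; BP_Checkpoint is a checkpoint actor that registers as cleared when exited in its forward direction, marked by its author as possibly not working.
; End overlap on Trigger casts the other actor to PlayerController, then dots its velocity with the Arrow's forward vector.
; A positive result calls CheckpointCleared with the checkpoint number, unhides Checkpoint and Trigger, shows CheckpointClearedFB, disables further overlaps and prints a debug string.
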(event OnComponentEndOverlap(Trigger)
  (params (OverlappedComponent :type Primitive%20Component%20Object%20Reference) (OtherActor :type Actor%20Object%20Reference) (OtherComp :type Primitive%20Component%20Object%20Reference) (OtherBodyIndex :type Integer))
  ;[1 1 1] Checkpoint System - Cleared when overlapping ends. - NOT SURE IF THIS IS WORKING.
  (bind _asplayer_controller (Utilities|Casting|CastToPlayerController OtherActor))
  (if (> (Math|Vector|DotProduct (Transformation|GetVelocity _asplayer_controller) (Math|Rotator|GetRotationXVector (Transformation|GetWorldRotation (Variables|Default|GetArrow)))) 0.0)
    (Default|CallCheckpointCleared (Variables|Default|GetCheckpointNumber))
    (Development|SetHiddeninGame (Variables|Default|GetCheckpoint) false false)
    (Rendering|SetVisibility (Variables|Default|GetCheckpointClearedFB) true false)
    (Variables|/Script/Engine.PrimitiveComponent|SetbGenerateOverlapEvents (Variables|Default|GetTrigger) false)
    (Development|PrintString "Hello")))

(fn ConstructionScript)