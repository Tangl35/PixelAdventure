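; BP_InteractiveSpeed is a speed pickup that temporarily boosts the walk speed of an overlapping BP_PlayerBase.
; Any actor overlap destroys the flipbook and collider components before the player cast, leaving the actor alive to run the timer.
; The player's MaxWalkSpeed is raised relative to current max speed, then set to a fixed value after a delay, not restored.
; The Interact function is empty.
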(event EventBeginPlay
  (|CallParentFunction) ; This node is disabled and will not be called.\nDrag off pins to build functionality.
)

(event Collision|EventActorBeginOverlap
  (params (OtherActor :type Actor%20Object%20Reference))
  (Components|DestroyComponent (Variables|Default|GetPaperFlipbook))
  (bind _asbp_player_base (Utilities|Casting|CastToBP_PlayerBase OtherActor))
  (Variables|/Script/Engine.CharacterMovementComponent|SetMaxWalkSpeed (Variables|/Script/Engine.Character|GetCharacterMovement _asbp_player_base) (+ 3e+02 (Class|MovementComponent|GetMaxSpeed (Variables|/Script/Engine.Character|GetCharacterMovement _asbp_player_base))))
  (Utilities|FlowControl|Delay 5.0)
  (Variables|/Script/Engine.CharacterMovementComponent|SetMaxWalkSpeed (Variables|/Script/Engine.Character|GetCharacterMovement _asbp_player_base) 6e+02))

(fn ConstructionScript
  (|CallParentFunction))

(fn Interact
  (params (PlayerRef :type BP%20Player%20Base%20Object%20Reference)))